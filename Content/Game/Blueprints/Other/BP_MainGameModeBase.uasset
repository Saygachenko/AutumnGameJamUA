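; Game mode Blueprint that populates the level with enemies when play begins.
; SpawnEnemy gathers all BP_SpawnPoint actors, then spawns MaxEnemy BP_Enemy actors at randomly picked points, taking each enemy's scale from its point.
; Each used point is removed from the local array and destroyed so it is not picked again, and the Enemy variable keeps only the last spawn.
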(event `self.ReceiveBeginPlay`
  (`self.SpawnEnemy`))

(fn `SpawnEnemy`
  (locals (LocalArraySpawns :type "Array of /Game/Game/Blueprints/Other/BP_SpawnPoint Object Reference") (LocalSpawn :type "/Game/Game/Blueprints/Other/BP_SpawnPoint Object Reference"))
  (bind _outactors (`GameplayStatics.GetAllActorsOfClass` "/Game/Game/Blueprints/Other/BP_SpawnPoint.BP_SpawnPoint_C"))
  (set `local.LocalArraySpawns` _outactors)
  (for _ (range (`self.MaxEnemy`))
    (set `local.LocalSpawn` (`KismetArrayLibrary.Array_Random` (`local.LocalArraySpawns`)))
    (bind _returnvalue (`|SpawnActorFromClass` "/Game/Game/Blueprints/AI/BP_Enemy.BP_Enemy_C" (`KismetMathLibrary.MakeTransform` (`self.K2_GetActorLocation` (`local.LocalSpawn`)) (struct) (`/Game/Game/Blueprints/Other/BP_SpawnPoint.EnemyScale` (`local.LocalSpawn`))) "AdjustIfPossibleButAlwaysSpawn" "MultiplyWithRoot" null null))
    (set `self.Enemy` _returnvalue)
    (`KismetArrayLibrary.Array_RemoveItem` (`local.LocalArraySpawns`) (`local.LocalSpawn`))
    (`self.K2_DestroyActor` (`local.LocalSpawn`))))

(fn `UserConstructionScript`)