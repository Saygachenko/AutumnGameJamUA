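; Enemy ball AI that acts as hunter or victim depending on its scale relative to the player's BP_MainBall.
; At BeginPlay it picks an enemy or victim material by that comparison, then patrols random reachable points.
; On sensing the player, it flees if the player is larger on all axes, otherwise chases and destroys the player on reaching it.
; Fleeing repeatedly targets random points offset along the line to the player by RunAwayDistance.
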(event `self.ReceiveBeginPlay`
  (`self.SetMaterialSpawning`)
  (bind _asbp_main_ball (cast `/Game/Game/Blueprints/Character/BP_MainBall` (`GameplayStatics.GetPlayerPawn` 0)))
  (set `self.MainBall` _asbp_main_ball)
  (`self.AIPatrol`))

(event `self.AIPerception.OnTargetPerceptionUpdated`
  (params (Actor :type "Actor Object Reference") (Stimulus :type "AIStimulus Structure"))
  (bind _returnvalue (`self.GetTransform`))
  (bind _returnvalue_2 (`self.GetTransform` (`self.MainBall`)))
  (if Stimulus_bSuccessfullySensed
    (if (== Actor (`self.MainBall`))
      (if (and (> (.x (.scale _returnvalue_2)) (.x (.scale _returnvalue))) (> (.y (.scale _returnvalue_2)) (.y (.scale _returnvalue))) (> (.z (.scale _returnvalue_2)) (.z (.scale _returnvalue))))
        (`self.RunAway`)
        (else
          (`self.Investigation`))))
    (else
      (`self.AIPatrol`))))

(event `AIPatrol`
  (set `CharacterMovementComponent.MaxWalkSpeed` 300.0 (`self.CharacterMovement`))
  (`|AIMoveTo` self (`NavigationSystemV1.K2_GetRandomReachablePointInRadius` (`self.K2_GetActorLocation`) 1500.0 null null) null
    (:`OnSuccess`
      _)
    (:`OnFail`
      _))
  (`self.AIPatrol`))

(event `RunAway`
  (bind (_returnvalue_x _returnvalue_y _returnvalue_z) (`KismetMathLibrary.BreakVector` (`self.K2_GetActorLocation`)))
  (set `CharacterMovementComponent.MaxWalkSpeed` 500.0 (`self.CharacterMovement`))
  (`|AIMoveTo` self (`NavigationSystemV1.K2_GetRandomReachablePointInRadius` (`KismetMathLibrary.MakeVector` (.x (+ (`self.K2_GetActorLocation`) (* (`KismetMathLibrary.GetForwardVector` (`KismetMathLibrary.FindLookAtRotation` (`self.K2_GetActorLocation`) (`self.K2_GetActorLocation` (`self.MainBall`)))) (`self.RunAwayDistance`)))) (.y (+ (`self.K2_GetActorLocation`) (* (`KismetMathLibrary.GetForwardVector` (`KismetMathLibrary.FindLookAtRotation` (`self.K2_GetActorLocation`) (`self.K2_GetActorLocation` (`self.MainBall`)))) (`self.RunAwayDistance`)))) _returnvalue_z) 500.0 null null) null
    (:`OnSuccess`
      _)
    (:`OnFail`
      _))
  (`self.RunAway`))

(event `Investigation`
  (set `CharacterMovementComponent.MaxWalkSpeed` 400.0 (`self.CharacterMovement`))
  (`|AIMoveTo` self (0.0 0.0 0.0) (`self.MainBall`)
    (:`OnSuccess`
      (`self.K2_DestroyActor` (`self.MainBall`)))))

(fn `RunAways`
  (returns (Result :type "Vector Structure"))
  (bind (_returnvalue_x _returnvalue_y _returnvalue_z) (`KismetMathLibrary.BreakVector` (`self.K2_GetActorLocation`)))
  (return (`NavigationSystemV1.K2_GetRandomReachablePointInRadius` (`KismetMathLibrary.MakeVector` (.x (+ (`self.K2_GetActorLocation`) (* (`KismetMathLibrary.GetForwardVector` (`KismetMathLibrary.FindLookAtRotation` (`self.K2_GetActorLocation`) (`self.K2_GetActorLocation` (`self.MainBall`)))) (`self.RunAwayDistance`)))) (.y (+ (`self.K2_GetActorLocation`) (* (`KismetMathLibrary.GetForwardVector` (`KismetMathLibrary.FindLookAtRotation` (`self.K2_GetActorLocation`) (`self.K2_GetActorLocation` (`self.MainBall`)))) (`self.RunAwayDistance`)))) _returnvalue_z) 500.0 null null)))

(fn `SetMaterialSpawning`
  (bind _returnvalue (`self.GetTransform`))
  (bind _returnvalue_2 (`self.GetTransform` (`GameplayStatics.GetPlayerPawn` 0)))
  (if (and (<= (.x (.scale _returnvalue_2)) (.x (.scale _returnvalue))) (<= (.y (.scale _returnvalue_2)) (.y (.scale _returnvalue))) (<= (.z (.scale _returnvalue_2)) (.z (.scale _returnvalue))))
    (`PrimitiveComponent.SetMaterial` (`self.Sphere`) 0 "/Game/Game/Materials/NPC_Colors/M_MrEnemy.M_MrEnemy")
    (else
      (`PrimitiveComponent.SetMaterial` (`self.Sphere`) 0 "/Game/Game/Materials/NPC_Colors/M_MrVictim.M_MrVictim"))))

(fn `UserConstructionScript`)